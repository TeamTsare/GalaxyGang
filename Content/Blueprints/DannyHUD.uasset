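; DannyHUD sets up the player's UI and level save data at BeginPlay, forcing Stage to 1 on every start.
; LoadSaveInstance loads or creates the LevelData save, initializes it on first use and saves it back.
; It creates MainHUD and a hidden Starpad_Menu, and RefSet cross-links them with CharacterDanny and LevelData.
; The save object itself receives a MainHUD reference, then runs SelectWorld.
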(event `self.ReceiveBeginPlay`
  (bind _returnvalue (`GameplayStatics.GetPlayerController` 0))
  (bind (_leveldata _saveinstance) (`self.LoadSaveInstance`))
  (set `/Game/Blueprints/SaveBluprints/LevelData.Stage#` 1 _leveldata)
  (`KismetSystemLibrary.PrintString` (`KismetStringLibrary.Conv_IntToString` (`/Game/Blueprints/SaveBluprints/LevelData.Stage#` _leveldata)))
  (bind _returnvalue_2 (`|CreateWidget` "/Game/Blueprints/Widgets/Starpad_Menu.Starpad_Menu_C" _returnvalue _saveinstance))
  (bind _returnvalue_3 (`|CreateWidget` "/Game/Blueprints/Widgets/MainHUD.MainHUD_C" _returnvalue false false _returnvalue_2))
  (bind _ascharacter_danny (cast `/Game/Characters/Char_Danny/CharacterDanny` (`GameplayStatics.GetPlayerCharacter` 0)))
  (bind _leveldata_2 (`self.RefSet` _returnvalue_3 _ascharacter_danny _leveldata _returnvalue_2))
  (`UserWidget.AddToViewport` _returnvalue_3 0)
  (`UserWidget.AddToViewport` _returnvalue_2 0)
  (`Widget.SetVisibility` _returnvalue_2 "Hidden")
  (`/Game/Blueprints/SaveBluprints/LevelData.SelectWorld` _leveldata_2))

(fn `UserConstructionScript`)