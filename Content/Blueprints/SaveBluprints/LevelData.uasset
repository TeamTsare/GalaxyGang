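; LevelData Blueprint that turns World and Stage numbers into display names for the HUD.
; SelectWorld sets WorldName and calls that world's event, which picks StageName by Stage and runs SetNames to pass itself to MainHud's StartHud.
; Only worlds 1 and 2 are wired through; events for worlds 3 to 7 are unfinished, never reached from SelectWorld or linked to SetNames, and several stage names sit disconnected.
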(event `GalaxyOfDreams`
  ;[1 1 1] World 1
  (switch `int` (`self.Stage#`)
    (:`1`
      (set `self.StageName` "Fountain Island"))
    (:`2`
      (set `self.StageName` "Bits 'N' Pieces")))
  (`self.SetNames`))

(event `Copse Treehouse Cluster`
  ;[1 1 1] World 7
  (switch `int` (`self.Stage#`)
    (:`1`
      (set `self.StageName` "Tree Town"))))

(event `SelectWorld`
  (switch `int` (`self.World#`)
    (:`0`
      (set `self.WorldName` ""))
    (:`1`
      (set `self.WorldName` "Galaxy Of Dreams")
      (`self.GalaxyOfDreams`))
    (:`2`
      (set `self.WorldName` "Pirate'sPlanet")
      (`self.PiratePlanet`))))

(event `PiratePlanet`
  ;[1 1 1] World 2
  (switch `int` (`self.Stage#`)
    (:`1`
      (set `self.StageName` "Buccaneer Beach"))
    (:`2`
      (set `self.StageName` "Captain's Cove"))
    (:`3`
      (set `self.StageName` "No-Beard's Noway"))
    (:`4`
      (set `self.StageName` "Inside No-Beard's Cavern"))
    (:`5`
      (set `self.StageName` "Shippy Shipyard")))
  (`self.SetNames`))

(event `SetNames`
  (`/Game/Blueprints/Widgets/MainHUD.StartHud` (`self.MainHud`) self))

(event `DryMoons`
  ;[1 1 1] World 3
  (switch `int` (`self.Stage#`)
    (:`1`
      (set `self.StageName` "Coliseum"))
    (:`2`
      (set `self.StageName` "Clockwork Moon"))
    (:`3`
      (set `self.StageName` "Ruin Moon"))
    (:`4`
      (set `self.StageName` "Cinnamon Moon"))))

(event `RedArea`
  ;[1 1 1] World 4
  (switch `int` (`self.Stage#`)
    (:`1`
      (set `self.StageName` "Unknown Red Area"))))

(event `Detritus Junkyard Nebula`
  ;[1 1 1] World 5
  (switch `int` (`self.Stage#`)
    (:`1`
      (set `self.StageName` "Crash SIte"))))

(event `GamblingGalaxy`
  ;[1 1 1] World 6
  (switch `int` (`self.Stage#`)
    (:`1`
      (set `self.StageName` "Sin City Satellite"))))