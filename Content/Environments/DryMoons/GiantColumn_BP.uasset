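; GiantColumn_BP is a Dry Moons environment column that floats up and down while slowly tumbling.
; BeginPlay stores the column's world Z as the center, and Tick offsets it with a time-based sine of amplitude and frequency, using degree-based Sind on a 2π-scaled angle.
; Tick also adds a fixed local rotation each frame, independent of delta time.
; Doubloon pickup and older yaw-rotation logic remain disconnected and never run.
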(event `self.ReceiveBeginPlay`
  ;[1 1 1] Floating
  (set `self.Phase/Offset` (.z (`SceneComponent.K2_GetComponentLocation` (`self.Column`)))))

(event `self.ReceiveTick`
  (params (DeltaSeconds :type "Float (single-precision)"))
  ;[1 1 1] Rotation
  (`|ExecutionSequence`
    (:`then_0`
      ;[1 1 1] Floating
      (`SceneComponent.K2_SetWorldLocation` (`self.Column`) (`KismetMathLibrary.MakeVector` (.x (`SceneComponent.K2_GetComponentLocation` (`self.Column`))) (.y (`SceneComponent.K2_GetComponentLocation` (`self.Column`))) (+ (* (`self.Amptitude`) (`KismetMathLibrary.DegSin` (* (`self.Frequency`) (`KismetMathLibrary.MultiplyByPi` 2.0) (`GameplayStatics.GetTimeSeconds`)))) (`self.Phase/Offset`))) false false))
    (:`then_1`
      ;[1 1 1] New Rotation
      (`SceneComponent.K2_AddLocalRotation` (`self.Column`) (struct :`Pitch` 0.25 :`Yaw` 0.25) false false) ; AddLocalRotation for Rotating on X and Y
    )))

(event `self.ReceiveActorBeginOverlap`
  (params (OtherActor :type "Actor Object Reference")))

(fn `UserConstructionScript`)