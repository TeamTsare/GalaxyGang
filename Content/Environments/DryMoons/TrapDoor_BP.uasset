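; Trap door for the DryMoons environment that slides open when the player character's OpenTest flag is set.
; BeginPlay caches the world locations of the Door, Midway and End components.
; Tick polls the flag on CharacterDanny and plays a timeline that lerps the door straight from start to end, without sweep.
; An unconnected two-stage timeline chain through the midway point never runs.
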(event `self.ReceiveBeginPlay`
  (set `self.StartLoc` (`SceneComponent.K2_GetComponentLocation` (`self.Door`)))
  (set `self.MidLoc` (`SceneComponent.K2_GetComponentLocation` (`self.Midway`)))
  (set `self.EndLoc` (`SceneComponent.K2_GetComponentLocation` (`self.End`))))

(event `self.ReceiveTick`
  (params (DeltaSeconds :type "Float (single-precision)"))
  (bind _ascharacter_danny (cast `/Game/Characters/Char_Danny/CharacterDanny` (`GameplayStatics.GetPlayerCharacter` 0)))
  (if (`/Game/Characters/Char_Danny/CharacterDanny.OpenTest` _ascharacter_danny)
    (bind (_direction _newtrack_0) (`Timeline|Timeline_3`)
      (:`Update`
        (`SceneComponent.K2_SetWorldLocation` (`self.Door`) (`KismetMathLibrary.VLerp` (`self.StartLoc`) (`self.EndLoc`) _newtrack_0) false false)))))

(fn `UserConstructionScript`)