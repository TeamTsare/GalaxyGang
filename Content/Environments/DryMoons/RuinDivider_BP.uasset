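; RuinDivider_BP is a ruin divider whose Wall component slides toward an End component's position when the player's OpenTest flag is set.
; BeginPlay caches the world locations of Wall and End.
; Tick polls OpenTest on the CharacterDanny player and plays a timeline that lerps the Wall between those points.
; The cached world-space positions are applied through SetRelativeLocation, without sweep, and nothing reverses the movement.
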(event `self.ReceiveBeginPlay`
  (set `self.StartLoc` (`SceneComponent.K2_GetComponentLocation` (`self.Wall`)))
  (set `self.EndLoc` (`SceneComponent.K2_GetComponentLocation` (`self.End`))))

(event `self.ReceiveTick`
  (params (DeltaSeconds :type "Float (single-precision)"))
  (bind _ascharacter_danny (cast `/Game/Characters/Char_Danny/CharacterDanny` (`GameplayStatics.GetPlayerCharacter` 0)))
  (if (`/Game/Characters/Char_Danny/CharacterDanny.OpenTest` _ascharacter_danny)
    (bind (_direction _newtrack_0) (`Timeline|Timeline_0`)
      (:`Update`
        (`SceneComponent.K2_SetRelativeLocation` (`self.Wall`) (`KismetMathLibrary.VLerp` (`self.StartLoc`) (`self.EndLoc`) _newtrack_0) false false)))))

(fn `UserConstructionScript`)