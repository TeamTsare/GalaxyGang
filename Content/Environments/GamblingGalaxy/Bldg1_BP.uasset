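; Building Blueprint for the Gambling Galaxy environment that animates cycling colored lights on its PLACE mesh.
; On BeginPlay it loops forever, calling Change2, Change1 and Change3 with a one-second Delay after each.
; Each function sets three material slots to a different rotation of Blue, Red and Yellow, producing a chasing color effect.
; The loop is a Delay chain wired back to its start rather than a timer or Tick.
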(event `self.ReceiveBeginPlay`
  (`self.Change2` :!label _label)
  (`KismetSystemLibrary.Delay` 1.0)
  (`self.Change1`)
  (`KismetSystemLibrary.Delay` 1.0)
  (`self.Change3`)
  (`KismetSystemLibrary.Delay` 1.0)
  (goto _label))

(fn `Change1`
  (bind _place (`self.PLACE`))
  (`|ExecutionSequence`
    (:`then_0`
      (`PrimitiveComponent.SetMaterial` _place 3 (`self.Blue`)))
    (:`then_1`
      (`PrimitiveComponent.SetMaterial` _place 4 (`self.Red`)))
    (:`then_2`
      (`PrimitiveComponent.SetMaterial` _place 5 (`self.Yellow`)))))

(fn `Change2`
  (bind _place (`self.PLACE`))
  (`|ExecutionSequence`
    (:`then_0`
      (`PrimitiveComponent.SetMaterial` _place 3 (`self.Yellow`)))
    (:`then_1`
      (`PrimitiveComponent.SetMaterial` _place 4 (`self.Blue`)))
    (:`then_2`
      (`PrimitiveComponent.SetMaterial` _place 5 (`self.Red`)))))

(fn `Change3`
  (bind _place (`self.PLACE`))
  (`|ExecutionSequence`
    (:`then_0`
      (`PrimitiveComponent.SetMaterial` _place 3 (`self.Red`)))
    (:`then_1`
      (`PrimitiveComponent.SetMaterial` _place 4 (`self.Yellow`)))
    (:`then_2`
      (`PrimitiveComponent.SetMaterial` _place 5 (`self.Blue`)))))

(fn `UserConstructionScript`)