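; VIP environment Blueprint for the Gambling Galaxy area that animates three stair pieces by endlessly swapping their materials.
; From BeginPlay, a sequence starts three looping chains, one per stair, each setting material slot 1 to one of three variants with a shared BetweenTime delay.
; The first and third stairs cycle their variants in descending order while the middle one runs ascending.
; The construction script and StairA function are empty.
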(event `self.ReceiveBeginPlay`
  (bind _betweentime (`self.BetweenTime`))
  (bind _betweentime_2 (`self.BetweenTime`))
  (bind _betweentime_3 (`self.BetweenTime`))
  (`|ExecutionSequence`
    (:`then_0`
      (`PrimitiveComponent.SetMaterial` (`self.Stair1`) 1 (`self.MatA3`) :!label _label)
      (`KismetSystemLibrary.Delay` _betweentime_2)
      (`PrimitiveComponent.SetMaterial` (`self.Stair1`) 1 (`self.MatA2`))
      (`KismetSystemLibrary.Delay` _betweentime_2)
      (`PrimitiveComponent.SetMaterial` (`self.Stair1`) 1 (`self.MatA1`))
      (`KismetSystemLibrary.Delay` _betweentime_2)
      (goto _label))
    (:`then_1`
      (`PrimitiveComponent.SetMaterial` (`self.Stair2`) 1 (`self.MatB1`) :!label _label_2)
      (`KismetSystemLibrary.Delay` _betweentime_3)
      (`PrimitiveComponent.SetMaterial` (`self.Stair2`) 1 (`self.MatB2`))
      (`KismetSystemLibrary.Delay` _betweentime_3)
      (`PrimitiveComponent.SetMaterial` (`self.Stair2`) 1 (`self.MatB3`))
      (`KismetSystemLibrary.Delay` _betweentime_3)
      (goto _label_2))
    (:`then_2`
      (`PrimitiveComponent.SetMaterial` (`self.Stair3`) 1 (`self.MatC3`) :!label _label_3)
      (`KismetSystemLibrary.Delay` _betweentime)
      (`PrimitiveComponent.SetMaterial` (`self.Stair3`) 1 (`self.MatC2`))
      (`KismetSystemLibrary.Delay` _betweentime)
      (`PrimitiveComponent.SetMaterial` (`self.Stair3`) 1 (`self.MatC1`))
      (`KismetSystemLibrary.Delay` _betweentime)
      (goto _label_3))))

(fn `StairA`)

(fn `UserConstructionScript`)