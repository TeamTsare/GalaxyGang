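; Neon tree prop for the Gambling Galaxy environment that applies materials to its Tree component in a timed sequence.
; BeginPlay runs an endless latent loop that sets six material slots one after another, with a fixed Delay after each.
; Each slot always receives its own material variable, so later passes reapply the same assignments unless those variables change elsewhere.
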(event `self.ReceiveBeginPlay`
  (bind _tree (`self.Tree`))
  (`PrimitiveComponent.SetMaterial` _tree 0 (`self.Mat1`) :!label _label)
  (`KismetSystemLibrary.Delay` 3.0)
  (`PrimitiveComponent.SetMaterial` _tree 1 (`self.Mat2`))
  (`KismetSystemLibrary.Delay` 3.0)
  (`PrimitiveComponent.SetMaterial` _tree 2 (`self.Mat3`))
  (`KismetSystemLibrary.Delay` 3.0)
  (`PrimitiveComponent.SetMaterial` _tree 3 (`self.Mat4`))
  (`KismetSystemLibrary.Delay` 3.0)
  (`PrimitiveComponent.SetMaterial` _tree 4 (`self.Mat5`))
  (`KismetSystemLibrary.Delay` 3.0)
  (`PrimitiveComponent.SetMaterial` _tree 5 (`self.Mat6`))
  (`KismetSystemLibrary.Delay` 3.0)
  (goto _label))

(fn `UserConstructionScript`)