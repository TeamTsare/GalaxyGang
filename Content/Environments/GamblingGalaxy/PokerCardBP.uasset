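; Animated Gambling Galaxy poker card prop that floats up and down while its faces light up in turn.
; BeginPlay runs two endless delay loops: one cycles Ace, King, Jack, 1 and all-cards highlights, the other blinks a separate material slot yellow.
; Each highlight function swaps the mesh's material slots between glow and black materials.
; Tick applies a sine-wave Z offset around the height captured at BeginPlay.
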(event `self.ReceiveBeginPlay`
  (`|ExecutionSequence`
    (:`then_0`
      (`self.ToAce` null :!label _label)
      (`KismetSystemLibrary.Delay` 2.0)
      (`self.ToKing` null)
      (`KismetSystemLibrary.Delay` 2.0)
      (`self.ToJack` null)
      (`KismetSystemLibrary.Delay` 2.0)
      (`self.To1` null)
      (`KismetSystemLibrary.Delay` 2.0)
      (`self.AllCards`)
      (`KismetSystemLibrary.Delay` 2.0)
      (goto _label))
    (:`then_1`
      (`KismetSystemLibrary.Delay` 3.0 :!label _label_2)
      (`PrimitiveComponent.SetMaterial` (`self.Poker`) 1 (`self.GlowYellow`))
      (`KismetSystemLibrary.Delay` 3.0)
      (`PrimitiveComponent.SetMaterial` (`self.Poker`) 1 (`self.BlackMat`))
      (goto _label_2))
    (:`then_2`
      ;[1 1 1] Floating
      (set `self.Phase/Offset` (.z (`SceneComponent.K2_GetComponentLocation` (`self.Poker`)))))))

(event `self.ReceiveTick`
  (params (DeltaSeconds :type "Float (single-precision)"))
  ;[1 1 1] Floating
  (`SceneComponent.K2_SetWorldLocation` (`self.Poker`) (`KismetMathLibrary.MakeVector` (.x (`SceneComponent.K2_GetComponentLocation` (`self.Poker`))) (.y (`SceneComponent.K2_GetComponentLocation` (`self.Poker`))) (+ (* (`self.Amptitude`) (`KismetMathLibrary.DegSin` (* (`self.Frequency`) (`KismetMathLibrary.MultiplyByPi` 2.0) (`GameplayStatics.GetTimeSeconds`)))) (`self.Phase/Offset`))) false false))

(fn `AllCards`
  (bind _poker (`self.Poker`))
  (bind _glowred (`self.GlowRed`))
  (bind _glowblack (`self.GlowBlack`))
  (`|ExecutionSequence`
    (:`then_0`
      (`PrimitiveComponent.SetMaterial` _poker 0 _glowred))
    (:`then_1`
      (`PrimitiveComponent.SetMaterial` _poker 2 _glowblack))
    (:`then_2`
      (`PrimitiveComponent.SetMaterial` _poker 3 _glowblack))
    (:`then_3`
      (`PrimitiveComponent.SetMaterial` _poker 4 _glowred))))

(fn `To1`
  (params (Material :type "MaterialInterface Object Reference"))
  (bind _poker (`self.Poker`))
  (bind _blackmat (`self.BlackMat`))
  (`|ExecutionSequence`
    (:`then_0`
      (`PrimitiveComponent.SetMaterial` _poker 0 _blackmat))
    (:`then_1`
      (`PrimitiveComponent.SetMaterial` _poker 2 _blackmat))
    (:`then_2`
      (`PrimitiveComponent.SetMaterial` _poker 3 (`self.GlowBlack`)))
    (:`then_3`
      (`PrimitiveComponent.SetMaterial` _poker 4 _blackmat))))

(fn `ToAce`
  (params (Material :type "MaterialInterface Object Reference"))
  (bind _poker (`self.Poker`))
  (bind _blackmat (`self.BlackMat`))
  (`|ExecutionSequence`
    (:`then_0`
      (`PrimitiveComponent.SetMaterial` _poker 0 (`self.GlowRed`)))
    (:`then_1`
      (`PrimitiveComponent.SetMaterial` _poker 2 _blackmat))
    (:`then_2`
      (`PrimitiveComponent.SetMaterial` _poker 3 _blackmat))
    (:`then_3`
      (`PrimitiveComponent.SetMaterial` _poker 4 _blackmat))))

(fn `ToJack`
  (params (Material :type "MaterialInterface Object Reference"))
  (bind _poker (`self.Poker`))
  (bind _blackmat (`self.BlackMat`))
  (`|ExecutionSequence`
    (:`then_0`
      (`PrimitiveComponent.SetMaterial` _poker 0 _blackmat))
    (:`then_1`
      (`PrimitiveComponent.SetMaterial` _poker 2 _blackmat))
    (:`then_2`
      (`PrimitiveComponent.SetMaterial` _poker 3 _blackmat))
    (:`then_3`
      (`PrimitiveComponent.SetMaterial` _poker 4 (`self.GlowRed`)))))

(fn `ToKing`
  (params (Material :type "MaterialInterface Object Reference"))
  (bind _poker (`self.Poker`))
  (bind _blackmat (`self.BlackMat`))
  (`|ExecutionSequence`
    (:`then_0`
      (`PrimitiveComponent.SetMaterial` _poker 0 _blackmat))
    (:`then_1`
      (`PrimitiveComponent.SetMaterial` _poker 2 (`self.GlowBlack`)))
    (:`then_2`
      (`PrimitiveComponent.SetMaterial` _poker 3 _blackmat))
    (:`then_3`
      (`PrimitiveComponent.SetMaterial` _poker 4 _blackmat))))

(fn `UserConstructionScript`)