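; NeonColumnBP is a decorative neon column for the Gambling Galaxy environment that animates by switching materials.
; From BeginPlay, an endless Delay-driven loop swaps the first material slot of Column2 through Neon3, Neon2 and Neon1 at a fixed interval of just over a second.
; The construction script is empty.
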(event `self.ReceiveBeginPlay`
  (`PrimitiveComponent.SetMaterial` (`self.Column2`) 0 (`self.Neon3`) :!label _label)
  (`KismetSystemLibrary.Delay` 1.2)
  (`PrimitiveComponent.SetMaterial` (`self.Column2`) 0 (`self.Neon2`))
  (`KismetSystemLibrary.Delay` 1.2)
  (`PrimitiveComponent.SetMaterial` (`self.Column2`) 0 (`self.Neon1`))
  (`KismetSystemLibrary.Delay` 1.2)
  (goto _label))

(fn `UserConstructionScript`)