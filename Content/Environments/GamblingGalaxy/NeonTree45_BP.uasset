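; Animated neon tree prop for the Gambling Galaxy environment that cycles its coloured stems in an endless light show.
; BeginPlay runs a Delay-driven loop that lights the red, green, blue, yellow and pink stems one at a time, then flashes all of them repeatedly.
; Each step function swaps On/Off materials per slot on the Tree mesh; only the all-on and all-off steps also set a sixth slot, using pink.
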(event `self.ReceiveBeginPlay`
  (`self.Stem1` :!label _label)
  (`KismetSystemLibrary.Delay` 1.0)
  (`self.Stem2`)
  (`KismetSystemLibrary.Delay` 1.0)
  (`self.Stem3`)
  (`KismetSystemLibrary.Delay` 1.0)
  (`self.Stem4`)
  (`KismetSystemLibrary.Delay` 1.0)
  (`self.Stem5`)
  (`KismetSystemLibrary.Delay` 1.0)
  (`self.StemOn`)
  (`KismetSystemLibrary.Delay` 0.3)
  (`self.StemOff`)
  (`KismetSystemLibrary.Delay` 0.3)
  (`self.StemOn`)
  (`KismetSystemLibrary.Delay` 0.3)
  (`self.StemOff`)
  (`KismetSystemLibrary.Delay` 0.3)
  (`self.StemOn`)
  (`KismetSystemLibrary.Delay` 0.3)
  (`self.StemOff`)
  (`KismetSystemLibrary.Delay` 0.3)
  (`self.StemOn`)
  (`KismetSystemLibrary.Delay` 0.3)
  (`self.StemOff`)
  (`KismetSystemLibrary.Delay` 0.3)
  (goto _label))

(fn `Stem1`
  (`|ExecutionSequence`
    (:`then_0`
      (`PrimitiveComponent.SetMaterial` (`self.Tree`) 0 (`self.RedOn`)))
    (:`then_1`
      (`PrimitiveComponent.SetMaterial` (`self.Tree`) 1 (`self.GreenOff`)))
    (:`then_2`
      (`PrimitiveComponent.SetMaterial` (`self.Tree`) 2 (`self.BlueOff`)))
    (:`then_3`
      (`PrimitiveComponent.SetMaterial` (`self.Tree`) 3 (`self.YellowOff`)))
    (:`then_4`
      (`PrimitiveComponent.SetMaterial` (`self.Tree`) 4 (`self.PinkOff`)))))

(fn `Stem2`
  (`|ExecutionSequence`
    (:`then_0`
      (`PrimitiveComponent.SetMaterial` (`self.Tree`) 0 (`self.RedOff`)))
    (:`then_1`
      (`PrimitiveComponent.SetMaterial` (`self.Tree`) 1 (`self.GreenOn`)))
    (:`then_2`
      (`PrimitiveComponent.SetMaterial` (`self.Tree`) 2 (`self.BlueOff`)))
    (:`then_3`
      (`PrimitiveComponent.SetMaterial` (`self.Tree`) 3 (`self.YellowOff`)))
    (:`then_4`
      (`PrimitiveComponent.SetMaterial` (`self.Tree`) 4 (`self.PinkOff`)))))

(fn `Stem3`
  (`|ExecutionSequence`
    (:`then_0`
      (`PrimitiveComponent.SetMaterial` (`self.Tree`) 0 (`self.RedOff`)))
    (:`then_1`
      (`PrimitiveComponent.SetMaterial` (`self.Tree`) 1 (`self.GreenOff`)))
    (:`then_2`
      (`PrimitiveComponent.SetMaterial` (`self.Tree`) 2 (`self.BlueOn`)))
    (:`then_3`
      (`PrimitiveComponent.SetMaterial` (`self.Tree`) 3 (`self.YellowOff`)))
    (:`then_4`
      (`PrimitiveComponent.SetMaterial` (`self.Tree`) 4 (`self.PinkOff`)))))

(fn `Stem4`
  (`|ExecutionSequence`
    (:`then_0`
      (`PrimitiveComponent.SetMaterial` (`self.Tree`) 0 (`self.RedOff`)))
    (:`then_1`
      (`PrimitiveComponent.SetMaterial` (`self.Tree`) 1 (`self.GreenOff`)))
    (:`then_2`
      (`PrimitiveComponent.SetMaterial` (`self.Tree`) 2 (`self.BlueOff`)))
    (:`then_3`
      (`PrimitiveComponent.SetMaterial` (`self.Tree`) 3 (`self.YellowOn`)))
    (:`then_4`
      (`PrimitiveComponent.SetMaterial` (`self.Tree`) 4 (`self.PinkOff`)))))

(fn `Stem5`
  (`|ExecutionSequence`
    (:`then_0`
      (`PrimitiveComponent.SetMaterial` (`self.Tree`) 0 (`self.RedOff`)))
    (:`then_1`
      (`PrimitiveComponent.SetMaterial` (`self.Tree`) 1 (`self.GreenOff`)))
    (:`then_2`
      (`PrimitiveComponent.SetMaterial` (`self.Tree`) 2 (`self.BlueOff`)))
    (:`then_3`
      (`PrimitiveComponent.SetMaterial` (`self.Tree`) 3 (`self.YellowOff`)))
    (:`then_4`
      (`PrimitiveComponent.SetMaterial` (`self.Tree`) 4 (`self.PinkOn`)))))

(fn `StemOff`
  (`|ExecutionSequence`
    (:`then_0`
      (`PrimitiveComponent.SetMaterial` (`self.Tree`) 0 (`self.RedOff`)))
    (:`then_1`
      (`PrimitiveComponent.SetMaterial` (`self.Tree`) 1 (`self.GreenOff`)))
    (:`then_2`
      (`PrimitiveComponent.SetMaterial` (`self.Tree`) 2 (`self.BlueOff`)))
    (:`then_3`
      (`PrimitiveComponent.SetMaterial` (`self.Tree`) 3 (`self.YellowOff`)))
    (:`then_4`
      (`|ExecutionSequence`
        (:`then_0`
          (`PrimitiveComponent.SetMaterial` (`self.Tree`) 4 (`self.PinkOff`)))
        (:`then_1`
          (`PrimitiveComponent.SetMaterial` (`self.Tree`) 5 (`self.PinkOff`)))))))

(fn `StemOn`
  (`|ExecutionSequence`
    (:`then_0`
      (`PrimitiveComponent.SetMaterial` (`self.Tree`) 0 (`self.RedOn`)))
    (:`then_1`
      (`PrimitiveComponent.SetMaterial` (`self.Tree`) 1 (`self.GreenOn`)))
    (:`then_2`
      (`PrimitiveComponent.SetMaterial` (`self.Tree`) 2 (`self.BlueOn`)))
    (:`then_3`
      (`PrimitiveComponent.SetMaterial` (`self.Tree`) 3 (`self.YellowOn`)))
    (:`then_4`
      (`|ExecutionSequence`
        (:`then_0`
          (`PrimitiveComponent.SetMaterial` (`self.Tree`) 4 (`self.PinkOn`)))
        (:`then_1`
          (`PrimitiveComponent.SetMaterial` (`self.Tree`) 5 (`self.PinkOn`)))))))

(fn `UserConstructionScript`)