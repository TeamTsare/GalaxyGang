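; FunBP is a Gambling Galaxy environment actor that animates the glow on its Fun mesh like a flashing sign.
; From BeginPlay, an endless delay-driven loop lights four material slots in yellow, blue, purple, green order, then flashes them together.
; OffGlow and OnGlow swap all slots between the off material and their colors.
; The sine-based floating logic is disconnected, and Blink is never called.
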(event `self.ReceiveBeginPlay`
  (`self.OffGlow` null :!label _label)
  (`KismetSystemLibrary.Delay` 1.5)
  (`PrimitiveComponent.SetMaterial` (`self.Fun`) 1 (`self.GlowYellow`))
  (`KismetSystemLibrary.Delay` 1.5)
  (`PrimitiveComponent.SetMaterial` (`self.Fun`) 2 (`self.GlowBlue`))
  (`KismetSystemLibrary.Delay` 1.5)
  (`PrimitiveComponent.SetMaterial` (`self.Fun`) 3 (`self.GlowPurple`))
  (`KismetSystemLibrary.Delay` 1.5)
  (`PrimitiveComponent.SetMaterial` (`self.Fun`) 0 (`self.GlowGreen`))
  (`KismetSystemLibrary.Delay` 1.5)
  (`self.OffGlow` null)
  (`KismetSystemLibrary.Delay` 0.2)
  (`self.OnGlow` null)
  (`KismetSystemLibrary.Delay` 0.2)
  (`self.OffGlow` null)
  (`KismetSystemLibrary.Delay` 0.2)
  (`self.OnGlow` null)
  (`KismetSystemLibrary.Delay` 0.2)
  (`self.OffGlow` null)
  (`KismetSystemLibrary.Delay` 0.2)
  (`self.OnGlow` null)
  (`KismetSystemLibrary.Delay` 0.2)
  (goto _label))

(event `self.ReceiveTick`
  (params (DeltaSeconds :type "Float (single-precision)")))

(fn `Blink`
  (`self.OffGlow` null))

(fn `OffGlow`
  (params (Material :type "MaterialInterface Object Reference"))
  (bind _fun (`self.Fun`))
  (bind _offmat (`self.OffMat`))
  (`|ExecutionSequence`
    (:`then_0`
      (`PrimitiveComponent.SetMaterial` _fun 0 _offmat))
    (:`then_1`
      (`PrimitiveComponent.SetMaterial` _fun 1 _offmat))
    (:`then_2`
      (`PrimitiveComponent.SetMaterial` _fun 2 _offmat))
    (:`then_3`
      (`PrimitiveComponent.SetMaterial` _fun 3 _offmat))))

(fn `OnGlow`
  (params (Material :type "MaterialInterface Object Reference"))
  (bind _fun (`self.Fun`))
  (`|ExecutionSequence`
    (:`then_0`
      (`PrimitiveComponent.SetMaterial` _fun 0 (`self.GlowGreen`)))
    (:`then_1`
      (`PrimitiveComponent.SetMaterial` _fun 1 (`self.GlowYellow`)))
    (:`then_2`
      (`PrimitiveComponent.SetMaterial` _fun 2 (`self.GlowBlue`)))
    (:`then_3`
      (`PrimitiveComponent.SetMaterial` _fun 3 (`self.GlowPurple`)))))

(fn `UserConstructionScript`)