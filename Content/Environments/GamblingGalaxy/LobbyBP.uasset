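; LobbyBP is a Gambling Galaxy environment actor that animates neon on its Lobby component.
; From BeginPlay, an endless Delay loop swaps one material slot through three neon materials at a fixed interval, producing a repeating sign-like flicker cycle.
; The construction script is empty.
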(event `self.ReceiveBeginPlay`
  (`PrimitiveComponent.SetMaterial` (`self.Lobby`) 2 (`self.Neon3`) :!label _label)
  (`KismetSystemLibrary.Delay` 0.4)
  (`PrimitiveComponent.SetMaterial` (`self.Lobby`) 2 (`self.Neon2`))
  (`KismetSystemLibrary.Delay` 0.4)
  (`PrimitiveComponent.SetMaterial` (`self.Lobby`) 2 (`self.Neon1`))
  (`KismetSystemLibrary.Delay` 0.4)
  (goto _label))

(fn `UserConstructionScript`)