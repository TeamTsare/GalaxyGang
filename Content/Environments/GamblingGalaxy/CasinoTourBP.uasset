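; CasinoTourBP is a Gambling Galaxy environment Blueprint that makes its static mesh float up and down.
; BeginPlay stores the mesh's starting world Z as PhaseOffset, the center of the bob.
; Every Tick sets world Z to that offset plus an Amptitude-scaled sine of game time, keeping X and Y unchanged.
; Frequency is multiplied by 2π but fed into the degree-based Sind, so it is not in hertz.
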(event `self.ReceiveTick`
  (params (DeltaSeconds :type "Float (single-precision)"))
  ;[1 1 1] Floating
  (`SceneComponent.K2_SetWorldLocation` (`self.StaticMesh`) (`KismetMathLibrary.MakeVector` (.x (`SceneComponent.K2_GetComponentLocation` (`self.StaticMesh`))) (.y (`SceneComponent.K2_GetComponentLocation` (`self.StaticMesh`))) (+ (* (`self.Amptitude`) (`KismetMathLibrary.DegSin` (* (`self.Frequency`) (`KismetMathLibrary.MultiplyByPi` 2.0) (`GameplayStatics.GetTimeSeconds`)))) (`self.Phase/Offset`))) false false))

(event `self.ReceiveBeginPlay`
  ;[1 1 1] Floating
  (set `self.Phase/Offset` (.z (`SceneComponent.K2_GetComponentLocation` (`self.StaticMesh`)))))

(fn `UserConstructionScript`)