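; RavineBP is a Gambling Galaxy environment Blueprint that animates a ravine by swapping its material over time.
; From BeginPlay, an endless loop sets the first material slot of the Ravine component through three materials in a back-and-forth order, with a fixed delay between swaps.
; The loop is a latent Delay chain wired back to its start, so it needs no Tick or timer.
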(event `self.ReceiveBeginPlay`
  (bind _ravine (`self.Ravine`))
  (`PrimitiveComponent.SetMaterial` _ravine 0 (`self.Mat1`) :!label _label)
  (`KismetSystemLibrary.Delay` 1.0)
  (`PrimitiveComponent.SetMaterial` _ravine 0 (`self.Mat2`))
  (`KismetSystemLibrary.Delay` 1.0)
  (`PrimitiveComponent.SetMaterial` _ravine 0 (`self.Mat3`))
  (`KismetSystemLibrary.Delay` 1.0)
  (`PrimitiveComponent.SetMaterial` _ravine 0 (`self.Mat2`))
  (`KismetSystemLibrary.Delay` 1.0)
  (goto _label))

(fn `UserConstructionScript`)