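; Animated floating BINGO sign prop for the Gambling Galaxy environment.
; BeginPlay runs an endless delayed loop that lights one letter at a time by swapping glow and black materials per mesh slot, then lights every slot together before restarting.
; Tick bobs the mesh vertically on a sine of game time around its starting height, captured in BeginPlay's second Sequence pin.
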(event `self.ReceiveTick`
  (params (DeltaSeconds :type "Float (single-precision)"))
  ;[1 1 1] Floating
  (`SceneComponent.K2_SetWorldLocation` (`self.BINGO`) (`KismetMathLibrary.MakeVector` (.x (`SceneComponent.K2_GetComponentLocation` (`self.BINGO`))) (.y (`SceneComponent.K2_GetComponentLocation` (`self.BINGO`))) (+ (* (`self.Amptitude`) (`KismetMathLibrary.DegSin` (* (`self.Frequency`) (`KismetMathLibrary.MultiplyByPi` 2.0) (`GameplayStatics.GetTimeSeconds`)))) (`self.Phase/Offset`))) false false))

(event `self.ReceiveBeginPlay`
  ;[1 1 1] Floating
  (`|ExecutionSequence`
    (:`then_0`
      (`self.ToB` null :!label _label)
      (`KismetSystemLibrary.Delay` 1.0)
      (`self.ToI` null)
      (`KismetSystemLibrary.Delay` 1.0)
      (`self.ToN` null)
      (`KismetSystemLibrary.Delay` 1.0)
      (`self.ToG` null)
      (`KismetSystemLibrary.Delay` 1.0)
      (`self.ToO` null)
      (`KismetSystemLibrary.Delay` 1.0)
      (`self.To!` null)
      (`KismetSystemLibrary.Delay` 1.0)
      (goto _label))
    (:`then_1`
      (set `self.Phase/Offset` (.z (`SceneComponent.K2_GetComponentLocation` (`self.BINGO`)))))))

(fn `To!`
  (params (Material :type "MaterialInterface Object Reference"))
  (bind _bingo (`self.BINGO`))
  (bind _glowmat (`self.GlowMat`))
  (`|ExecutionSequence`
    (:`then_0`
      (`PrimitiveComponent.SetMaterial` _bingo 0 _glowmat))
    (:`then_1`
      (`PrimitiveComponent.SetMaterial` _bingo 1 _glowmat))
    (:`then_2`
      (`PrimitiveComponent.SetMaterial` _bingo 2 _glowmat))
    (:`then_3`
      (`PrimitiveComponent.SetMaterial` _bingo 3 _glowmat))
    (:`then_4`
      (`PrimitiveComponent.SetMaterial` _bingo 4 _glowmat))
    (:`then_5`
      (`PrimitiveComponent.SetMaterial` _bingo 5 _glowmat))))

(fn `ToB`
  (params (Material :type "MaterialInterface Object Reference"))
  (bind _bingo (`self.BINGO`))
  (bind _blackmat (`self.BlackMat`))
  (`|ExecutionSequence`
    (:`then_0`
      (`PrimitiveComponent.SetMaterial` _bingo 0 (`self.GlowMat`)))
    (:`then_1`
      (`PrimitiveComponent.SetMaterial` _bingo 1 _blackmat))
    (:`then_2`
      (`PrimitiveComponent.SetMaterial` _bingo 2 _blackmat))
    (:`then_3`
      (`PrimitiveComponent.SetMaterial` _bingo 3 _blackmat))
    (:`then_4`
      (`PrimitiveComponent.SetMaterial` _bingo 4 _blackmat))
    (:`then_5`
      (`PrimitiveComponent.SetMaterial` _bingo 5 _blackmat))))

(fn `ToG`
  (params (Material :type "MaterialInterface Object Reference"))
  (bind _bingo (`self.BINGO`))
  (bind _blackmat (`self.BlackMat`))
  (`|ExecutionSequence`
    (:`then_0`
      (`PrimitiveComponent.SetMaterial` _bingo 0 _blackmat))
    (:`then_1`
      (`PrimitiveComponent.SetMaterial` _bingo 1 _blackmat))
    (:`then_2`
      (`PrimitiveComponent.SetMaterial` _bingo 2 _blackmat))
    (:`then_3`
      (`PrimitiveComponent.SetMaterial` _bingo 3 _blackmat))
    (:`then_4`
      (`PrimitiveComponent.SetMaterial` _bingo 4 _blackmat))
    (:`then_5`
      (`PrimitiveComponent.SetMaterial` _bingo 5 (`self.GlowMat`)))))

(fn `ToI`
  (params (Material :type "MaterialInterface Object Reference"))
  (bind _bingo (`self.BINGO`))
  (bind _blackmat (`self.BlackMat`))
  (`|ExecutionSequence`
    (:`then_0`
      (`PrimitiveComponent.SetMaterial` _bingo 0 _blackmat))
    (:`then_1`
      (`PrimitiveComponent.SetMaterial` _bingo 1 (`self.GlowMat`)))
    (:`then_2`
      (`PrimitiveComponent.SetMaterial` _bingo 2 _blackmat))
    (:`then_3`
      (`PrimitiveComponent.SetMaterial` _bingo 3 _blackmat))
    (:`then_4`
      (`PrimitiveComponent.SetMaterial` _bingo 4 _blackmat))
    (:`then_5`
      (`PrimitiveComponent.SetMaterial` _bingo 5 _blackmat))))

(fn `ToN`
  (params (Material :type "MaterialInterface Object Reference"))
  (bind _bingo (`self.BINGO`))
  (bind _blackmat (`self.BlackMat`))
  (`|ExecutionSequence`
    (:`then_0`
      (`PrimitiveComponent.SetMaterial` _bingo 0 _blackmat))
    (:`then_1`
      (`PrimitiveComponent.SetMaterial` _bingo 1 _blackmat))
    (:`then_2`
      (`PrimitiveComponent.SetMaterial` _bingo 2 _blackmat))
    (:`then_3`
      (`PrimitiveComponent.SetMaterial` _bingo 3 (`self.GlowMat`)))
    (:`then_4`
      (`PrimitiveComponent.SetMaterial` _bingo 4 _blackmat))
    (:`then_5`
      (`PrimitiveComponent.SetMaterial` _bingo 5 _blackmat))))

(fn `ToO`
  (params (Material :type "MaterialInterface Object Reference"))
  (bind _bingo (`self.BINGO`))
  (bind _blackmat (`self.BlackMat`))
  (`|ExecutionSequence`
    (:`then_0`
      (`PrimitiveComponent.SetMaterial` _bingo 0 _blackmat))
    (:`then_1`
      (`PrimitiveComponent.SetMaterial` _bingo 1 _blackmat))
    (:`then_2`
      (`PrimitiveComponent.SetMaterial` _bingo 2 (`self.GlowMat`)))
    (:`then_3`
      (`PrimitiveComponent.SetMaterial` _bingo 3 _blackmat))
    (:`then_4`
      (`PrimitiveComponent.SetMaterial` _bingo 4 _blackmat))
    (:`then_5`
      (`PrimitiveComponent.SetMaterial` _bingo 5 _blackmat))))

(fn `UserConstructionScript`)