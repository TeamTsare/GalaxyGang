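; World 1 object in the hideout hub that spins, bobs on a sine wave around its starting height, and offers a world selection menu.
; Overlap with UICollision by CharacterDanny sets Near and shows a prompt widget rotated toward the camera; leaving hides both widget and menu.
; BeginPlay creates the hidden WorldSelection widget and registers this actor on the character.
; ToggleWidgetVisibility_WorldSelection toggles that menu only while Near.
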(event `self.ReceiveTick`
  (params (DeltaSeconds :type "Float (single-precision)"))
  (bind _w1 (`self.W1`))
  (bind _widget (`self.Widget`))
  (bind _w1_2 (`self.W1`))
  (`|ExecutionSequence`
    (:`then_0`
      ;[1 1 1] Rotate
      (bind _output_get (set `self.Rotate` (+ (`self.RotateBy`) (.yaw (`SceneComponent.K2_GetComponentRotation` _w1_2)))))
      (`SceneComponent.K2_SetWorldRotation` _w1_2 (`KismetMathLibrary.MakeRotator` (.roll (`SceneComponent.K2_GetComponentRotation` _w1_2)) (.pitch (`SceneComponent.K2_GetComponentRotation` _w1_2)) _output_get) false false))
    (:`then_1`
      ;[1 1 1] FaceCamera
      (`SceneComponent.K2_SetWorldRotation` _widget (.rotation (`self.GetTransform` (`GameplayStatics.GetPlayerController` 0))) false false)
      (`SceneComponent.K2_AddLocalRotation` _widget (struct :`Yaw` -180.0) false false))
    (:`then_2`
      ;[1 1 1] Floating
      (`SceneComponent.K2_SetWorldLocation` _w1 (`KismetMathLibrary.MakeVector` (.x (`SceneComponent.K2_GetComponentLocation` _w1)) (.y (`SceneComponent.K2_GetComponentLocation` _w1)) (+ (* (`self.Amptitude`) (`KismetMathLibrary.DegSin` (* (`self.Frequency`) (`KismetMathLibrary.MultiplyByPi` 2.0) (`GameplayStatics.GetTimeSeconds`)))) (`self.Phase/Offset`))) false false))))

(event `self.UICollision.OnComponentBeginOverlap`
  (params (OverlappedComponent :type "PrimitiveComponent Object Reference") (OtherActor :type "Actor Object Reference") (OtherComp :type "PrimitiveComponent Object Reference") (OtherBodyIndex :type Integer) (bFromSweep :type Boolean) (SweepResult :type "HitResult Structure (by ref)"))
  (cast `/Game/Characters/Char_Danny/CharacterDanny` OtherActor)
  (`SceneComponent.SetVisibility` (`self.Widget`) true false) ; check means visible
  (set `self.Near` true))

(event `self.UICollision.OnComponentEndOverlap`
  (params (OverlappedComponent :type "PrimitiveComponent Object Reference") (OtherActor :type "Actor Object Reference") (OtherComp :type "PrimitiveComponent Object Reference") (OtherBodyIndex :type Integer))
  (cast `/Game/Characters/Char_Danny/CharacterDanny` OtherActor)
  (`SceneComponent.SetVisibility` (`self.Widget`) false false) ; check means visible
  (set `self.Near` false)
  (`Widget.SetVisibility` (`self.WorldSelection`) "Hidden"))

(event `self.ReceiveBeginPlay`
  (`|ExecutionSequence`
    (:`then_0`
      ;[1 1 1] Floating
      (set `self.Phase/Offset` (.z (`SceneComponent.K2_GetComponentLocation` (`self.W1`)))))
    (:`then_1`
      (`SceneComponent.SetVisibility` (`self.Widget`) false false) ; check means visible
      (bind _returnvalue (`|CreateWidget` "/Game/Blueprints/Widgets/WorldSelection.WorldSelection_C" (`GameplayStatics.GetPlayerController` 0)))
      (bind _output_get (set `self.WorldSelection` _returnvalue))
      (`UserWidget.AddToViewport` _output_get 0)
      (`Widget.SetVisibility` (`self.WorldSelection`) "Hidden" :!label _label))
    (:`then_2`
      (bind _ascharacter_danny (cast `/Game/Characters/Char_Danny/CharacterDanny` (`GameplayStatics.GetPlayerCharacter` 0)))
      (set `/Game/Characters/Char_Danny/CharacterDanny.World1BP_CD` self _ascharacter_danny))))

(event `self.Hitbox.OnComponentBeginOverlap`
  (params (OverlappedComponent :type "PrimitiveComponent Object Reference") (OtherActor :type "Actor Object Reference") (OtherComp :type "PrimitiveComponent Object Reference") (OtherBodyIndex :type Integer) (bFromSweep :type Boolean) (SweepResult :type "HitResult Structure (by ref)")))

(event `self.Hitbox.OnComponentEndOverlap`
  (params (OverlappedComponent :type "PrimitiveComponent Object Reference") (OtherActor :type "Actor Object Reference") (OtherComp :type "PrimitiveComponent Object Reference") (OtherBodyIndex :type Integer)))

(event `ToggleWidgetVisibility_WorldSelection`
  (bind _worldselection (`self.WorldSelection`))
  (if (`self.Near`)
    (if (`Widget.IsVisible` _worldselection)
      (goto _label)
      (else
        (`Widget.SetVisibility` _worldselection "Visible")))))

(fn `UserConstructionScript`)