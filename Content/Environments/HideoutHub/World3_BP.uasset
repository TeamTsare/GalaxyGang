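; World 3 selection object in the hideout hub, showing a rotating, floating world with a camera-facing name and prompt.
; Tick spins the mesh, bobs it and the name on a sine wave, and turns UI elements and collision toward the player.
; Overlap by CharacterDanny toggles the prompt or lock based on Locked, which also picks locked name widget or emissive glow.
; Lock evaluation and selection-menu creation are unwired; SetReference is empty.
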(event `self.ReceiveTick`
  (params (DeltaSeconds :type "Float (single-precision)"))
  (bind _w3 (`self.W3`))
  (bind _widget (`self.Widget`))
  (bind _w3_2 (`self.W3`))
  (bind _world_name (`self.World Name`))
  (bind _uicollision (`self.UICollision`))
  (bind _returnvalue (* (`self.Amptitude`) (`KismetMathLibrary.DegSin` (* (`self.Frequency`) (`KismetMathLibrary.MultiplyByPi` 2.0) (`GameplayStatics.GetTimeSeconds`)))))
  (`|ExecutionSequence`
    (:`then_0`
      ;[1 1 1] Rotate
      (bind _output_get (set `self.Rotate` (+ (`self.RotateBy`) (.yaw (`SceneComponent.K2_GetComponentRotation` _w3_2)))))
      (`SceneComponent.K2_SetWorldRotation` _w3_2 (`KismetMathLibrary.MakeRotator` (.roll (`SceneComponent.K2_GetComponentRotation` _w3_2)) (.pitch (`SceneComponent.K2_GetComponentRotation` _w3_2)) _output_get) false false))
    (:`then_1`
      ;[1 1 1] FaceCamera
      (`SceneComponent.K2_SetWorldRotation` _widget (.rotation (`self.GetTransform` (`GameplayStatics.GetPlayerController` 0))) false false)
      (`SceneComponent.K2_SetWorldRotation` (`self.Lock`) (.rotation (`self.GetTransform` (`GameplayStatics.GetPlayerController` 0))) false false)
      (`SceneComponent.K2_SetWorldRotation` (`self.World Name`) (.rotation (`self.GetTransform` (`GameplayStatics.GetPlayerController` 0))) false false)
      (`SceneComponent.K2_AddLocalRotation` _widget (struct :`Yaw` -180.0) false false)
      (`SceneComponent.K2_AddLocalRotation` (`self.Lock`) (struct :`Yaw` -180.0) false false)
      (`SceneComponent.K2_AddLocalRotation` (`self.World Name`) (struct :`Yaw` -180.0) false false)
      (`SceneComponent.K2_SetWorldRotation` _uicollision (`KismetMathLibrary.FindLookAtRotation` (`SceneComponent.K2_GetComponentLocation` _uicollision) (`KismetMathLibrary.MakeVector` (.x (`SceneComponent.K2_GetComponentLocation` (`Character.CapsuleComponent` (`GameplayStatics.GetPlayerCharacter` 0)))) (.y (`SceneComponent.K2_GetComponentLocation` (`Character.CapsuleComponent` (`GameplayStatics.GetPlayerCharacter` 0)))) (.z (`SceneComponent.K2_GetComponentLocation` (`self.Lock`))))) true false))
    (:`then_2`
      ;[1 1 1] Floating
      (`SceneComponent.K2_SetWorldLocation` _w3 (`KismetMathLibrary.MakeVector` (.x (`SceneComponent.K2_GetComponentLocation` _w3)) (.y (`SceneComponent.K2_GetComponentLocation` _w3)) (+ _returnvalue (`self.Phase/Offset`))) false false)
      (`SceneComponent.K2_SetWorldLocation` _world_name (`KismetMathLibrary.MakeVector` (.x (`SceneComponent.K2_GetComponentLocation` _world_name)) (.y (`SceneComponent.K2_GetComponentLocation` _world_name)) (+ _returnvalue (`self.WorldNameOffset`))) false false))))

(event `self.UICollision.OnComponentBeginOverlap`
  (params (OverlappedComponent :type "PrimitiveComponent Object Reference") (OtherActor :type "Actor Object Reference") (OtherComp :type "PrimitiveComponent Object Reference") (OtherBodyIndex :type Integer) (bFromSweep :type Boolean) (SweepResult :type "HitResult Structure (by ref)"))
  (cast `/Game/Characters/Char_Danny/CharacterDanny` OtherActor)
  (`SceneComponent.SetVisibility` (`KismetArrayLibrary.Array_Get` (`|MakeArray` (`self.Widget`) (`self.Lock`)) (`KismetMathLibrary.Conv_BoolToInt` (`self.Locked`))) true false) ; check means visible
  (set `self.Near` true))

(event `self.UICollision.OnComponentEndOverlap`
  (params (OverlappedComponent :type "PrimitiveComponent Object Reference") (OtherActor :type "Actor Object Reference") (OtherComp :type "PrimitiveComponent Object Reference") (OtherBodyIndex :type Integer))
  (cast `/Game/Characters/Char_Danny/CharacterDanny` OtherActor)
  (`SceneComponent.SetVisibility` (`KismetArrayLibrary.Array_Get` (`|MakeArray` (`self.Widget`) (`self.Lock`)) (`KismetMathLibrary.Conv_BoolToInt` (`self.Locked`))) false false) ; check means visible
  (set `self.Near` false))

(event `Floating`
  ;[1 1 1] Floating
  (set `self.Phase/Offset` (.z (`SceneComponent.K2_GetComponentLocation` (`self.W3`))))
  (set `self.WorldNameOffset` (.z (`SceneComponent.K2_GetComponentLocation` (`self.World Name`)))))

(event `SetLock/UnlockedState`
  ;[1 1 1] Set World State
  (if (`self.Locked`)
    (bind _returnvalue (`|CreateWidget` "/Game/Environments/HideoutHub/Widgets/LockedWorld3.LockedWorld3_C" (`GameplayStatics.GetPlayerController` 0)))
    (`WidgetComponent.SetWidget` (`self.World Name`) _returnvalue)
    (else
      (`MeshComponent.SetScalarParameterValueOnMaterials` (`self.W3`) "Emissive" 1.0))))

(event `self.ReceiveBeginPlay`
  ;[1 1 1] Event Begin Play
  (`|ExecutionSequence`
    (:`then_0`
      (`self.Floating`))
    (:`then_1`
      (`self.SetReference`))
    (:`then_2`
      (`self.SetLock/UnlockedState`))))

(event `SetReference`
  ;[1 1 1] Reference
)

(event `ToggleWidgetVisibility_WorldSelection`
  (bind _worldselection (`self.WorldSelection`))
  (if (`self.Near`)
    (if (`Widget.IsVisible` _worldselection)
      (`Widget.SetVisibility` _worldselection "Hidden")
      (else
        (`Widget.SetVisibility` _worldselection "Visible")))))

(fn `UserConstructionScript`)