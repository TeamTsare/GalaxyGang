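; Test actor Blueprint that endlessly cycles its static mesh through three materials.
; BeginPlay sets Mat1, Mat2 and Mat3 in turn on element 0, with a two-second Delay after each, then loops back to the first.
; An index-based selection using the Mat variable is left unconnected and never runs.
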(event `self.ReceiveBeginPlay`
  (`PrimitiveComponent.SetMaterial` (`self.StaticMesh`) 0 (`self.Mat1`) :!label _label)
  (`KismetSystemLibrary.Delay` 2.0)
  (`PrimitiveComponent.SetMaterial` (`self.StaticMesh`) 0 (`self.Mat2`))
  (`KismetSystemLibrary.Delay` 2.0)
  (`PrimitiveComponent.SetMaterial` (`self.StaticMesh`) 0 (`self.Mat3`))
  (`KismetSystemLibrary.Delay` 2.0)
  (goto _label))

(fn `UserConstructionScript`)